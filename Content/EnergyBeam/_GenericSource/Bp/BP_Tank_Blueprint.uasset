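; BP_Tank_Blueprint is an actor Blueprint in the EnergyBeam content that registers its Niagara beam and hit effect references at startup.
; BeginPlay fills two parallel, same-order arrays: Beams with five Niagara references and Hits with five NiagaraHit references.
; The graphs hold no firing or update logic, as Tick and overlap events are disabled and the construction script is empty.
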(event `self.ReceiveBeginPlay`
  (bind _beams (`self.Beams`))
  (bind _hits (`self.Hits`))
  (`KismetArrayLibrary.Array_Add` _beams (`self.Niagara1`))
  (`KismetArrayLibrary.Array_Add` _beams (`self.Niagara2`))
  (`KismetArrayLibrary.Array_Add` _beams (`self.Niagara3`))
  (`KismetArrayLibrary.Array_Add` _beams (`self.Niagara4`))
  (`KismetArrayLibrary.Array_Add` _beams (`self.Niagara5`))
  (`KismetArrayLibrary.Array_Add` _hits (`self.NiagaraHit01`))
  (`KismetArrayLibrary.Array_Add` _hits (`self.NiagaraHit02`))
  (`KismetArrayLibrary.Array_Add` _hits (`self.NiagaraHit03`))
  (`KismetArrayLibrary.Array_Add` _hits (`self.NiagaraHit04`))
  (`KismetArrayLibrary.Array_Add` _hits (`self.NiagaraHit05`)))

(fn `UserConstructionScript`)