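; Actor component that bridges the pawn and the dynamic radial menu UI on every instance except dedicated servers.
; On BeginPlay it creates the W_Menu widget, plus a demo W_Controls overlay, and binds the menu's event dispatchers.
; Pawn calls for toggling, paging, back, selection, thumbstick and input-device changes are forwarded to W_Menu.
; Selections return through HandleItemSelected, which switches on the stored menu enum and currently only prints the item name.
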(event `self.ReceiveBeginPlay`
  ;[0 0.2 1 0.25 14] Only proceed if it's a listen server or a client.
  (if (not (`KismetSystemLibrary.IsDedicatedServer`))
    ;[1 0 1 0.25 14] DELETE: UI controls / background. These buttons are not dynamic. This are just for demo purposes. The AXBY buttons as well as W_Controls widget is not needed and can be deleted altogether.
    (bind _returnvalue (`|CreateWidget` "/Game/DynamicRadialMenu/Widgets/W_Controls.W_Controls_C"))
    (bind _output_get (set `self.Controls` _returnvalue))
    (`UserWidget.AddToViewport` _output_get 0)
    ;[0 0.2 1 0.25 14] Create the main HUD container then bind to ItemSelected event dispatcher in W_Menu.
    (bind _returnvalue_2 (`|CreateWidget` "/Game/DynamicRadialMenu/Widgets/W_Menu.W_Menu_C"))
    (bind _output_get_2 (set `self.Menu` _returnvalue_2))
    (`UserWidget.AddToViewport` _output_get_2 0)
    (add `/Game/DynamicRadialMenu/Widgets/W_Menu.ItemSelected` (`self.Menu`) (`|CreateDelegate` :!event `HandleItemSelected`))
    ;[1 0 1 0.25 14] DELETE: This bind is called from the W_Menu event dispatcher. It simply toggles the visiblity of the controls by changing the icons / text in W_Controls.
    ;
    ; This is for demo purposes only and can be deleted.
    (add `/Game/DynamicRadialMenu/Widgets/W_Menu.DELETE ME - TOGGLE CONTROLS` (`self.Menu`) (`|CreateDelegate` :!event `UpdateControls`))))

(event `UpdateStyle`
  ;[1 0 1 0.25 14] This is for demo purposes only and can be deleted.
  (`/Game/DynamicRadialMenu/Widgets/W_Menu.DELETE ME - UpdateStyle` (`self.Menu`)))

(event `UpdateControls`
  (params (UseGamepad :type Boolean :default true) (`RadialMenuVisible?` :type Boolean :default true))
  ;[1 0 1 0.25 14] DELETE: This bind is called from the W_Menu event dispatcher. It simply toggles the visiblity of the controls by changing the icons / text in W_Controls.
  ;
  ; This is for demo purposes only and can be deleted.
  (`/Game/DynamicRadialMenu/Widgets/W_Controls.ToggleVisibility` (`self.Controls`) UseGamepad `RadialMenuVisible?`))

(fn `GamepadScroll`
  (params (`NextPage?` :type Boolean))
  ;[0 0.2 1 0.25 14] Called from the pawn when a gamepad button is pressed. Defaults are Left / Right Shoulder button (LB or RB on most controllers).
  ;
  ; LB = Previous Page (Next Page = false)
  ; RB = Next Page        (Next Page = true)
  (`/Game/DynamicRadialMenu/Widgets/W_Menu.GamepadScroll` (`self.Menu`) `NextPage?`))

(fn `GamepadSelect`
  ;[0 0.2 1 0.25 14] Called from the Pawn when the gamepad selection button is pressed. Default is Face Button Bottom (A or X on most controllers).
  ;
  ; We need to call this MakeSelection manually since the gamepad doesn't have an "on-click" event like a mouse. The mouse logic is handled in W_Menu itself in the OnMouseButtonDown override function.
  (`/Game/DynamicRadialMenu/Widgets/W_Menu.MakeSelection` (`self.Menu`)))

(fn `HandleItemSelected`
  (params (DisplayName :type Text))
  ;[0 0.2 1 0.25 14] This function is called from the W_Menu widget when the ItemSelected event dispatcher is called.
  ;
  ; The input can be anything you want it to be based on your own needs. Simply change what's being returned by the event dispatcher and add your logic to determine how to handle the selection.
  ;
  ; We switch on the menu to determine what menu was pulled up (crafting, skills, building, inventory, etc.) just to make it easier for us to determine what logic we need to do based on what menu was toggled.
  ;
  ; To add additional fields that you can pass back to this function, you can:
  ;
  ; 1) Update S_Menu to add any additional fields that you want your menu items to have,
  ; 2) Update the W_Menu -> ItemSelected event dispatcher to pass back the new fields,
  ; 3) Update this function to expect those new fields so that your binding event in the main event graph doesn't fail.
  ;
  ; Another option is you can simply get the display name or a unique ID sent to this function and use it to look up any additional data in separate data tables. This way your DT_Menu table won't get too cluttered with extra fields that aren't relevant to the radial menu and how the items are displayed.
  (switch `/Game/DynamicRadialMenu/Enums/E_Menus` (`self.SelectedMenu`)
    (:`NewEnumerator0`
      _)
    (:`NewEnumerator1`
      _)
    (:`NewEnumerator3`
      _))
  (`KismetSystemLibrary.PrintString` (`KismetTextLibrary.Conv_TextToString` (`local.DisplayName`))))

(fn `PreviousMenu`
  ;[0 0.2 1 0.25 14] Called from the pawn when a gamepad button is pressed. Default is Face Button Right (B or O on most controllers).
  (`/Game/DynamicRadialMenu/Widgets/W_Menu.PreviousMenu` (`self.Menu`)))

(fn `SetThumbstickValue`
  (params (X :type "Float (double-precision)") (Y :type "Float (double-precision)"))
  ;[0 0.2 1 0.25 14] This is called from the Pawn. We pass the X, Y values of the gamepad thumbstick to the menu. See the SetThumbstickAxes for more details.
  (`/Game/DynamicRadialMenu/Widgets/W_Menu.SetThumbstickAxes` (`self.Menu`) (`KismetMathLibrary.MakeVector2D` X Y)))

(fn `ToggleMenu`
  (params (Menu :type "/Game/DynamicRadialMenu/Enums/E_Menus Enum" :default "NewEnumerator2"))
  ;[0 0.2 1 0.25 14] This function is called from PP_Pawn. This is the function you need to call when toggling the menu.
  ;
  ; This input variable is of type enum E_Menus.
  ;
  ; We set this here because we use this later in HandleItemSelected to determine which menu we're dealing with.
  ;
  ; If you need a different "starting" or "top-level" menu, you need to:
  ;
  ; 1) Add the menu name to E_Menus,
  ; 2) Create a row in DT_Menu with that same name,
  ; 3) Bind a key in your pawn to call ToggleMenu passing it that new enum value.
  (set `self.SelectedMenu` Menu)
  ;[0 0.2 1 0.25 14] Pass the SelectedMenu to our Menu's ToggleMenu function to handle the population of menu items / showing / hiding the UI.
  (`/Game/DynamicRadialMenu/Widgets/W_Menu.ToggleMenu` (`self.Menu`) (`self.SelectedMenu`)))

(fn `UseGamepad`
  (params (UseGamepad :type Boolean))
  ;[0 0.2 1 0.25 14] Let the menu know whether the gamepad is being used or not. This is triggered from AnyKey event on the Pawn but can be replaced with your own logic - which you might want to do if you have some sort of character state management system.
  ;
  ; You might also want to have the player choose whether they want to use gamepad or mouse and lock them in to that choice until they change the setting. It's totally up to you. However, this asset is currently designed to allow swapping back and forth between the 2 peripherals seamlessly.
  (`/Game/DynamicRadialMenu/Widgets/W_Menu.UseGamepad` (`self.Menu`) UseGamepad)
  ;[1 0 1 0.25 14] DELETE: Not necessary - can be deleted and replaced with your own on-screen UI if you wish.
  ;
  ; This is just to change the visuals/text on the W_Controls widget to show you the controls.
  (`self.UpdateControls` (`local.UseGamepad`) (`/Game/DynamicRadialMenu/Widgets/W_Menu.ShowMenu` (`self.Menu`))))