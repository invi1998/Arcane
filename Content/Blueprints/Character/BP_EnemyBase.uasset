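; BP_EnemyBase is an enemy base Blueprint that handles dissolve effects and attack-agnostic facing through Motion Warping.
; Four events each play their own timeline for body, weapon, bow or arrow, driving the "Dissolve" scalar on a passed-in dynamic material instance.
; UpdateFacingTarget writes the given location to the "FacingTarget" warp target.
; BeginPlay, Tick, overlap and the construction script contain no logic.
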(event `self.ReceiveTick`
  (params (DeltaSeconds :type "Float (single-precision)")))

(event `self.StartDissolveTimeline`
  (params (DynamicMaterialInstance :type "MaterialInstanceDynamic Object Reference"))
  (bind (_direction _dissolvetrack) (`Timeline|DissolveTimeLine`)
    (:`Update`
      (`MaterialInstanceDynamic.SetScalarParameterValue` DynamicMaterialInstance "Dissolve" _dissolvetrack))))

(event `self.StartWeaponDissolveTimeline`
  (params (DynamicMaterialInstance :type "MaterialInstanceDynamic Object Reference"))
  (bind (_direction _weapondissolvetrack) (`Timeline|WeaponDissolveTimeLine`)
    (:`Update`
      (`MaterialInstanceDynamic.SetScalarParameterValue` DynamicMaterialInstance "Dissolve" _weapondissolvetrack))))

(event `self.StartBowDissolveTimeline`
  (params (DynamicMaterialInstance :type "MaterialInstanceDynamic Object Reference"))
  (bind (_direction _bowdissolvetrack) (`Timeline|BowDissolveTimeLine`)
    (:`Update`
      (`MaterialInstanceDynamic.SetScalarParameterValue` DynamicMaterialInstance "Dissolve" _bowdissolvetrack))))

(event `self.StartArrowDissolveTimeline`
  (params (DynamicMaterialInstance :type "MaterialInstanceDynamic Object Reference"))
  (bind (_direction _arrowdissolvetrack) (`Timeline|ArrowDissolveTimeLine`)
    (:`Update`
      (`MaterialInstanceDynamic.SetScalarParameterValue` DynamicMaterialInstance "Dissolve" _arrowdissolvetrack))))

(event `CombatInterface.UpdateFacingTarget`
  (params (Target :type "Vector Structure (by ref)"))
  (`MotionWarpingComponent.AddOrUpdateWarpTargetFromLocation` (`self.MotionWarping`) "FacingTarget" Target))

(fn `UserConstructionScript`)