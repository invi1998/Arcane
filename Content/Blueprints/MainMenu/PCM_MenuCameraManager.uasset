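; Main menu Player Camera Manager that frames registered focus targets selected by tag.
; UpdateFocusedTarget derives the desired camera pose from the target's transform, offset, arm length and rotation offset, with a fixed fallback location when none is valid.
; BlueprintUpdateCamera replaces the parent logic, applying that location instantly while interpolating rotation and returning TargetFOV.
; It also yaws the current target's listed actors toward the desired camera location each update.
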(event `/Game/Blueprints/MainMenu/Interface/Interface_MenuCameraManager.Update_FocusedTarget`
  (params (Tag :type Name))
  (bind _return_value (`self.FindActorToFocus` Tag))
  (bind (_tag _armlength _offset _rotationoffset _actorstofacecamera _selfreference) (break `/Game/Blueprints/MainMenu/Camera/Struct_FocusableCameraActor` _return_value))
  (bind (_returnvalue_location _returnvalue_rotation) (`KismetMathLibrary.BreakTransform` (`self.GetTransform` _selfreference)))
  (bind _returnvalue (+ _offset _returnvalue_location))
  (`/Engine/EditorBlueprintResources/StandardMacros.IsValid` _selfreference
    (:`Is Valid`
      (set `self.CurrentTarget` _return_value)
      (bind _output_get (set `self.DesiredCameraLocation` (+ _returnvalue (* (`KismetMathLibrary.GetForwardVector` _returnvalue_rotation) _armlength))))
      (set `self.DesiredCameraRotation` (`KismetMathLibrary.ComposeRotators` (`KismetMathLibrary.FindLookAtRotation` _output_get _returnvalue) _rotationoffset)))
    (:`Is Not Valid`
      (set `self.DesiredCameraLocation` (0.0 0.0 100.0)))))

(event `/Game/Blueprints/MainMenu/Interface/Interface_MenuCameraManager.Assign_FocusableTarget`
  (params (TargetInfo :type "/Game/Blueprints/MainMenu/Camera/Struct_FocusableCameraActor Structure"))
  (`KismetArrayLibrary.Array_Add` (`self.FocusableTargets`) TargetInfo))

(fn `BlueprintUpdateCamera`
  (params (CameraTarget :type "Actor Object Reference"))
  (returns (NewCameraLocation :type "Vector Structure") (NewCameraRotation :type "Rotator Structure") (NewCameraFOV :type "Float (single-precision)") (ReturnValue :type Boolean))
  (`|ExecutionSequence`
    (:`then_0`
      (for _array_element (`.ActorsToFaceCamera_21_3899F77A4838F99E0D3E7BB5B9638A89` (break `/Game/Blueprints/MainMenu/Camera/Struct_FocusableCameraActor` (`self.CurrentTarget`)))
        (bind (_returnvalue_roll _returnvalue_pitch _returnvalue_yaw) (`KismetMathLibrary.BreakRotator` (`KismetMathLibrary.FindLookAtRotation` (`self.K2_GetActorLocation` _array_element) (`self.DesiredCameraLocation`))))
        (`self.K2_SetActorRotation` _array_element (`KismetMathLibrary.MakeRotator` 0.0 0.0 (+ _returnvalue_yaw -90.0)) false)))
    (:`then_1`
      (set `self.TargetCamereRotation` (`KismetMathLibrary.RInterpTo` (`self.TargetCamereRotation`) (`self.DesiredCameraRotation`) (`GameplayStatics.GetWorldDeltaSeconds`) (`KismetMathLibrary.SafeDivide` 2.0 0.75))))
    (:`then_2`
      (return (`self.DesiredCameraLocation`) (`self.TargetCamereRotation`) (`self.TargetFOV`) true))))

(fn `FindActorToFocus`
  (params (Tag :type Name))
  (returns (`Return Value` :type "/Game/Blueprints/MainMenu/Camera/Struct_FocusableCameraActor Structure"))
  (locals (`Loc Target` :type "/Game/Blueprints/MainMenu/Camera/Struct_FocusableCameraActor Structure"))
  (for _array_element (`self.FocusableTargets`)
    (if (== (`.Tag_3_E5E26F704916A76FF9B27DB440EE5D80` (break `/Game/Blueprints/MainMenu/Camera/Struct_FocusableCameraActor` _array_element)) (`local.Tag`))
      (set `local.Loc Target` _array_element)
      (break)))
  (return (`local.Loc Target`)))

(fn `UserConstructionScript`)