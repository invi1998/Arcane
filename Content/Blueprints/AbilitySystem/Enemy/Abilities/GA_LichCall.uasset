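; Enemy summon ability, named for the Lich, that spawns random minions around the battlefield.
; Activation turns the avatar toward its combat target, shuffles spawn locations, marks each with a ground-summon Niagara effect and plays a random tagged attack montage.
; The montage's gameplay event starts a delayed loop that spawns minions one by one, facing away from the caster, each with a default controller.
; The graph never calls EndAbility.
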(event `self.K2_ActivateAbility`
  (bind _returnvalue (`self.GetAvatarActorFromActorInfo`))
  (bind _returnvalue_2 (+ (`|GetArrayItem` (`self.SpawnLocations`) (`self.SpawnLocationIndex`)) (0.0 0.0 70.0)))
  (bind _returnvalue_3 (message `EnemyInterface.GetCombatTarget` _returnvalue))
  (set `self.TargetLocation` (`Actor.K2_GetActorLocation` _returnvalue_3))
  (bind _ascombat_interface (cast `CombatInterface` _returnvalue))
  (`CombatInterface.UpdateFacingTarget` _ascombat_interface (`self.TargetLocation`))
  (bind _returnvalue_4 (message `CombatInterface.GetRandomAttackMontage` (`self.GetAvatarActorFromActorInfo`) (`self.Ability Tag`)))
  (bind (_abilitytag _montage _montagetag) (break `TaggedMontage` _returnvalue_4))
  (set `self.Montage Tag` _montagetag)
  (bind _returnvalue_5 (`self.GetSpawnLocations`))
  (bind _output_get (set `self.SpawnLocations` _returnvalue_5))
  (`KismetArrayLibrary.Array_Shuffle` _output_get)
  (for _array_element (`self.SpawnLocations`)
    (`NiagaraFunctionLibrary.SpawnSystemAtLocation` "/Game/Assets/Effects/Combat/NS_GroundSummon.NS_GroundSummon" _array_element))
  (`AbilityTask_PlayMontageAndWait.CreatePlayMontageAndWaitProxy` "None" _montage
    (:`then`
      (`AbilityTask_WaitGameplayEvent.WaitGameplayEvent` (`self.Montage Tag`) null
        (:`EventReceived`
          (if (< (`self.SpawnLocationIndex`) (`KismetArrayLibrary.Array_Length` (`self.SpawnLocations`))) :!label _label
            (bind _returnvalue_6 (`|SpawnActorFromClass` (`self.GetRandomMinionClass`) (`KismetMathLibrary.MakeTransform` _returnvalue_2 (`KismetMathLibrary.FindLookAtRotation` (`Actor.K2_GetActorLocation` (`self.GetAvatarActorFromActorInfo`)) _returnvalue_2)) "AlwaysSpawn" "MultiplyWithRoot" null null))
            (`Pawn.SpawnDefaultController` _returnvalue_6)
            (`/Engine/EditorBlueprintResources/StandardMacros.IncrementInt` (`self.SpawnLocationIndex`)
              (:`  `
                (`KismetSystemLibrary.Delay` 1.0)
                (goto _label)))))))))