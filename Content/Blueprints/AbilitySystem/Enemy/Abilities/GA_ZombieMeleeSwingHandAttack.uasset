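; Gameplay ability for a zombie enemy's melee hand-swing attack, which faces its combat target and plays a random attack montage.
; A montage swing-start event starts a fast looping timer that sphere-checks live players around the montage's combat socket, and the swing-end event stops it and ends the ability.
; Each player found is added to an ignore list to prevent repeat hits, and non-friendly ones take damage with a melee impact gameplay cue.
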(event `self.K2_ActivateAbility`
  (bind _returnvalue (`self.GetAvatarActorFromActorInfo`))
  (set `self.IgnoreActor` (`|MakeArray` _returnvalue))
  (bind _returnvalue_2 (message `EnemyInterface.GetCombatTarget` _returnvalue))
  (bind _ascombat_interface (cast `CombatInterface` _returnvalue))
  (`CombatInterface.UpdateFacingTarget` _ascombat_interface (`Actor.K2_GetActorLocation` _returnvalue_2))
  (bind _returnvalue_3 (message `CombatInterface.GetRandomAttackMontage` (`self.GetAvatarActorFromActorInfo`)))
  (bind (_montage _montagetag _impactsound _impacteffect) (break `TaggedMontage` _returnvalue_3))
  (set `self.Montage Tag` _montagetag)
  (set `self.Impact Sound` _impactsound)
  (set `self.Impact Effect` _impacteffect)
  (`AbilityTask_PlayMontageAndWait.CreatePlayMontageAndWaitProxy` "None" _montage 1.0 "None" false
    (:`then`
      (`AbilityTask_WaitGameplayEvent.WaitGameplayEvent` (struct :`TagName` "Event.Montage.Attack.HandSwingStart") null
        (:`then`
          (`AbilityTask_WaitGameplayEvent.WaitGameplayEvent` (struct :`TagName` "Event.Montage.Attack.HandSwingEnd") null
            (:`EventReceived`
              (`KismetSystemLibrary.K2_ClearAndInvalidateTimerHandle` (`self.SwingAttackTimerHandle`))
              (`KismetArrayLibrary.Array_Clear` (`self.IgnoreActor`))
              (`self.K2_EndAbility`))))
        (:`EventReceived`
          (`self.SwingAttack`))))
    (:`OnCompleted`
      (`self.K2_EndAbility` :!label _label))
    (:`OnInterrupted`
      (goto _label))
    (:`OnCancelled`
      (goto _label))))

(event `SwingAttack`
  (bind _returnvalue (`KismetSystemLibrary.K2_SetTimerDelegate` (delegate `SphereAttack`) 0.01 true))
  (set `self.SwingAttackTimerHandle` _returnvalue))

(event `SphereAttack`
  (bind _returnvalue (`self.GetAvatarActorFromActorInfo`))
  (bind _returnvalue_2 (`self.GetAvatarActorFromActorInfo`))
  (bind _returnvalue_3 (message `CombatInterface.GetCombatSocketLocation` _returnvalue_2 (`self.Montage Tag`)))
  (bind _outplayers (`AuraAbilitySystemLibrary.GetLivePlayerWithinRadius` _returnvalue_2 (`self.IgnoreActor`) _returnvalue_3 100.0))
  (for _array_element _outplayers
    (bind _returnvalue_4 (`AuraAbilitySystemLibrary.IsFriendly` (`self.GetAvatarActorFromActorInfo`) _array_element))
    (`KismetArrayLibrary.Array_Add` (`self.IgnoreActor`) _array_element)
    (if (not _returnvalue_4)
      (`self.CauseDamage` _array_element)
      (bind _returnvalue_5 (message `EnemyInterface.GetCombatTarget` _returnvalue))
      (`self.K2_ExecuteGameplayCueWithParams` (struct :`TagName` "GameplayCue.MeleeSwordImpact") (`AbilitySystemBlueprintLibrary.MakeGameplayCueParameters` 0.0 0.0 (struct) (struct) (struct) (`BlueprintGameplayTagLibrary.MakeGameplayTagContainerFromTag` (`self.Montage Tag`)) (struct) (`Actor.K2_GetActorLocation` _array_element) (0.0 0.0 0.0) null _returnvalue _returnvalue_5)))))