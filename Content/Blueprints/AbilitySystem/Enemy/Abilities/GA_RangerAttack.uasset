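; Gameplay ability for the skeleton archer enemy's ranged attack, firing a projectile at its combat target.
; On activation it updates the facing target through the combat interface and plays a random attack montage.
; The bow-shot gameplay event hides the held arrow and spawns a projectile toward the target's current location.
; The arrow reappears and the ability ends after a short delay, or when the montage completes, is interrupted or is cancelled.
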(event `self.K2_ActivateAbility`
  (bind _returnvalue (`self.GetAvatarActorFromActorInfo`))
  (bind _returnvalue_2 (message `EnemyInterface.GetCombatTarget` _returnvalue))
  (set `self.TargetLocation` (`Actor.K2_GetActorLocation` _returnvalue_2))
  (bind _ascombat_interface (cast `CombatInterface` _returnvalue))
  (`CombatInterface.UpdateFacingTarget` _ascombat_interface (`self.TargetLocation`))
  (bind _returnvalue_3 (message `CombatInterface.GetRandomAttackMontage` (`self.GetAvatarActorFromActorInfo`)))
  (bind (_montage _montagetag) (break `TaggedMontage` _returnvalue_3))
  (set `self.Montage Tag` _montagetag)
  (`AbilityTask_PlayMontageAndWait.CreatePlayMontageAndWaitProxy` "None" _montage
    (:`then`
      (`AbilityTask_WaitGameplayEvent.WaitGameplayEvent` (struct :`TagName` "Event.Montage.Attack.BowShotArrow") null
        (:`EventReceived`
          (bind _asbp_skeleton_bow (cast `/Game/Blueprints/Character/Skeleton_Bow/BP_SkeletonBow` (`self.GetAvatarActorFromActorInfo`)))
          (`SceneComponent.SetVisibility` (`AuraCharacterBase.BowArrow` _asbp_skeleton_bow) false true)
          (bind _returnvalue_4 (message `EnemyInterface.GetCombatTarget` (`self.GetAvatarActorFromActorInfo`)))
          (`self.SpawnProjectile` (`Actor.K2_GetActorLocation` _returnvalue_4))
          (`KismetSystemLibrary.Delay` 1.0)
          (bind _asbp_skeleton_bow_2 (cast `/Game/Blueprints/Character/Skeleton_Bow/BP_SkeletonBow` (`self.GetAvatarActorFromActorInfo`)))
          (`SceneComponent.SetVisibility` (`AuraCharacterBase.BowArrow` _asbp_skeleton_bow_2) true false)
          (`self.K2_EndAbility`))))
    (:`OnCompleted`
      (bind _asbp_skeleton_bow_3 (cast `/Game/Blueprints/Character/Skeleton_Bow/BP_SkeletonBow` (`self.GetAvatarActorFromActorInfo`) :!label _label))
      (`SceneComponent.SetVisibility` (`AuraCharacterBase.BowArrow` _asbp_skeleton_bow_3) true false)
      (`self.K2_EndAbility`))
    (:`OnInterrupted`
      (goto _label))
    (:`OnCancelled`
      (goto _label))))