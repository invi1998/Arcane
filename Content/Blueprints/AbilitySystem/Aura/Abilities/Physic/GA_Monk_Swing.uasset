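; Monk swing gameplay ability that faces the caster toward the point under the mouse and fires projectiles during a randomly chosen attack montage.
; Activation flags the weapon socket through an avatar message and takes the hit location from mouse target data.
; Two gameplay-event waits, armed together, each spawn projectiles toward that location on their MonkAttack montage event.
; Any montage exit clears the socket flag and ends the ability.
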(event `self.K2_ActivateAbility`
  (message `CombatInterface.UpdateWeaponSocket` (`self.GetAvatarActorFromActorInfo`) true)
  (bind (_asynctaskproxy _datahandle) (`TargetDataUnderMouse.CreateTargetDataUnderMouse`)
    (:`ValidData`
      (set `self.MouseHitLocation` (`.Location` (`GameplayStatics.BreakHitResult` (`AbilitySystemBlueprintLibrary.GetHitResultFromTargetData` _datahandle))))
      (message `CombatInterface.UpdateFacingTarget` (`self.GetAvatarActorFromActorInfo`) (`self.MouseHitLocation`))
      (`AbilityTask_PlayMontageAndWait.CreatePlayMontageAndWaitProxy` "None" (`KismetArrayLibrary.Array_Random` (`self.Montage to Play`))
        (:`then`
          (`AbilityTask_WaitGameplayEvent.WaitGameplayEvent` (struct :`TagName` "Event.Montage.Attack.MonkAttack1") null
            (:`then`
              (`AbilityTask_WaitGameplayEvent.WaitGameplayEvent` (struct :`TagName` "Event.Montage.Attack.MonkAttack2") null
                (:`EventReceived`
                  (`self.SpawnProjectiles` (`self.MouseHitLocation`) (`self.Socket Tag`)))))
            (:`EventReceived`
              (`self.SpawnProjectiles` (`self.MouseHitLocation`) (`self.Socket Tag`)))))
        (:`OnCompleted`
          (`self.PreEndAbility` :!label _label))
        (:`OnBlendOut`
          (goto _label))
        (:`OnInterrupted`
          (goto _label))
        (:`OnCancelled`
          (goto _label))))))

(fn `PreEndAbility`
  (message `CombatInterface.UpdateWeaponSocket` (`self.GetAvatarActorFromActorInfo`) false)
  (`self.K2_EndAbility`))