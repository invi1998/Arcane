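; Monk combo gameplay ability that faces the cursor target and plays a combo montage with weapon-trace melee damage.
; Montage gameplay events drive the steps: the first starts a looping trace timer, the second resets the hit-ignore list, the third stops tracing.
; Each tick sweeps line traces between previous and current sampled weapon points, damaging each non-friendly once per window and firing a gameplay cue.
; Montage completion, blend-out or interruption clears state and ends the ability.
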(event `self.K2_ActivateAbility`
  (bind (_asynctaskproxy _datahandle) (`TargetDataUnderMouse.CreateTargetDataUnderMouse`)
    (:`ValidData`
      (set `self.HitTargetLocation` (`.Location` (`GameplayStatics.BreakHitResult` (`AbilitySystemBlueprintLibrary.GetHitResultFromTargetData` _datahandle))))
      (set `self.IgnoreArray` (`|MakeArray` (`self.GetAvatarActorFromActorInfo`)))
      (message `CombatInterface.UpdateFacingTarget` (`self.GetAvatarActorFromActorInfo`) (`self.HitTargetLocation`))
      (`AbilityTask_PlayMontageAndWait.CreatePlayMontageAndWaitProxy` "None" "/Game/Blueprints/Character/Monk/Animation/Combo/AM_Combo2.AM_Combo2"
        (:`then`
          (`AbilityTask_WaitGameplayEvent.WaitGameplayEvent` (struct :`TagName` "Event.Montage.Combot.C2.Step1_start") null
            (:`then`
              (`AbilityTask_WaitGameplayEvent.WaitGameplayEvent` (struct :`TagName` "Event.Montage.Combot.C2.Step2_start") null
                (:`then`
                  (`AbilityTask_WaitGameplayEvent.WaitGameplayEvent` (struct :`TagName` "Event.Montage.Combot.C2.Step3_start") null
                    (:`EventReceived`
                      (`KismetArrayLibrary.Array_Clear` (`self.IgnoreArray`))
                      (set `self.IgnoreArray` (`|MakeArray` (`self.GetAvatarActorFromActorInfo`)))
                      (`KismetSystemLibrary.K2_ClearAndInvalidateTimerHandle` (`self.AttackTimerHandler`)))))
                (:`EventReceived`
                  (`KismetArrayLibrary.Array_Clear` (`self.IgnoreArray`))
                  (set `self.IgnoreArray` (`|MakeArray` (`self.GetAvatarActorFromActorInfo`))))))
            (:`EventReceived`
              (`self.StartAttackTrace`))))
        (:`OnCompleted`
          (`self.ClearAndEndAbility` :!label _label))
        (:`OnBlendOut`
          (goto _label))
        (:`OnInterrupted`
          (goto _label))
        (:`OnCancelled`
          (goto _label))))))

(event `StartAttackTrace`
  (bind _returnvalue (`self.GenerateAttackTraceSockets` (`self.TipSocket`) true -50.0 5 200.0))
  (set `self.Last_TipSocketLocations` _returnvalue)
  (bind _returnvalue_2 (`KismetSystemLibrary.K2_SetTimerDelegate` (delegate `TimerLineTrace`) 0.01 true))
  (set `self.AttackTimerHandler` _returnvalue_2))

(event `TimerLineTrace`
  (bind _returnvalue (`self.GetAvatarActorFromActorInfo`))
  (bind _returnvalue_2 (`self.GenerateAttackTraceSockets` (`self.TipSocket`) true -50.0 5 200.0))
  (bind _output_get (set `self.Current_TipSocketLocations` _returnvalue_2))
  (for (_array_element _array_index) _output_get
    (bind _outplayers (`AuraAbilitySystemLibrary.GetLivePlayerWithinRaycast` (`self.GetAvatarActorFromActorInfo`) (`self.IgnoreArray`) _array_element (`|GetArrayItem` (`self.Last_TipSocketLocations`) _array_index)))
    (for _array_element_2 _outplayers
      (bind _returnvalue_3 (`AuraAbilitySystemLibrary.IsFriendly` _array_element_2 (`self.GetAvatarActorFromActorInfo`)))
      (`KismetArrayLibrary.Array_Add` (`self.IgnoreArray`) _array_element_2)
      (if (not _returnvalue_3)
        (`self.CauseDamage` _array_element_2)
        (bind _returnvalue_4 (message `EnemyInterface.GetCombatTarget` _returnvalue))
        (`self.K2_ExecuteGameplayCueWithParams` (struct :`TagName` "GameplayCue.MonkCombo") (`AbilitySystemBlueprintLibrary.MakeGameplayCueParameters` 0.0 0.0 (struct) (struct) (struct) (struct) (struct) (0.0 0.0 0.0) (0.0 0.0 0.0) null _returnvalue _returnvalue_4)))))
  (`KismetArrayLibrary.Array_Clear` (`self.Last_TipSocketLocations`))
  (set `self.Last_TipSocketLocations` (`self.Current_TipSocketLocations`)))

(fn `ClearAndEndAbility`
  (`KismetArrayLibrary.Array_Clear` (`self.Last_TipSocketLocations`))
  (`KismetArrayLibrary.Array_Clear` (`self.Last_TailSocketLocations`))
  (`KismetArrayLibrary.Array_Clear` (`self.Current_TipSocketLocations`))
  (`KismetSystemLibrary.K2_ClearAndInvalidateTimerHandle` (`self.AttackTimerHandler`))
  (`self.K2_EndAbility`))