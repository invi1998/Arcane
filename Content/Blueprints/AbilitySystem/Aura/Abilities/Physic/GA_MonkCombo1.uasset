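; Monk first-combo melee ability: turns the avatar toward the cursor target, commits cost and plays a combo montage.
; The first montage event spawns VFX and starts a looping timer that raycasts between previous and current weapon tip and tail socket samples.
; Non-friendly hits take damage on authority, tip hits also firing a gameplay cue.
; Later step events reset the ignore list to allow re-hits; montage end clears the timer and commits cooldown.
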(event `SpawnRootVFX`
  (params (SystemTemplate :type "NiagaraSystem Object Reference"))
  (bind _returnvalue (`NiagaraFunctionLibrary.SpawnSystemAttached` SystemTemplate (`Actor.RootComponent` (`self.GetAvatarActorFromActorInfo`)) "None" (0.0 0.0 0.0) (struct) "KeepRelativeOffset" true))
  (set `self.RootVFX` _returnvalue))

(event `self.K2_ActivateAbility`
  (bind (_asynctaskproxy _datahandle) (`TargetDataUnderMouse.CreateTargetDataUnderMouse`)
    (:`ValidData`
      (set `self.HitTargetLocation` (`.Location` (`GameplayStatics.BreakHitResult` (`AbilitySystemBlueprintLibrary.GetHitResultFromTargetData` _datahandle))))
      (set `self.IgnoreArray` (`|MakeArray` (`self.GetAvatarActorFromActorInfo`)))
      (message `CombatInterface.UpdateFacingTarget` (`self.GetAvatarActorFromActorInfo`) (`self.HitTargetLocation`))
      (bind _returnvalue (`self.K2_CommitAbilityCost` false))
      (if _returnvalue
        (`AbilityTask_PlayMontageAndWait.CreatePlayMontageAndWaitProxy` "None" "/Game/Blueprints/Character/Monk/Animation/Combo/AM_Combo1.AM_Combo1"
          (:`then`
            (`AbilityTask_WaitGameplayEvent.WaitGameplayEvent` (struct :`TagName` "Event.Montage.Combot.c1.step1_start") null
              (:`then`
                (`AbilityTask_WaitGameplayEvent.WaitGameplayEvent` (struct :`TagName` "Event.Montage.Combot.c1.step2_start") null
                  (:`then`
                    (`AbilityTask_WaitGameplayEvent.WaitGameplayEvent` (struct :`TagName` "Event.Montage.Combot.c1.step3_start") null
                      (:`then`
                        (`AbilityTask_WaitGameplayEvent.WaitGameplayEvent` (struct :`TagName` "Event.Montage.Combot.c1.step4_start") null
                          (:`EventReceived`
                            (`KismetArrayLibrary.Array_Clear` (`self.IgnoreArray`))
                            (set `self.IgnoreArray` (`|MakeArray` (`self.GetAvatarActorFromActorInfo`))))))
                      (:`EventReceived`
                        (`KismetArrayLibrary.Array_Clear` (`self.IgnoreArray`))
                        (set `self.IgnoreArray` (`|MakeArray` (`self.GetAvatarActorFromActorInfo`))))))
                  (:`EventReceived`
                    (`KismetArrayLibrary.Array_Clear` (`self.IgnoreArray`))
                    (set `self.IgnoreArray` (`|MakeArray` (`self.GetAvatarActorFromActorInfo`))))))
              (:`EventReceived`
                (`self.StartAttackTrace`))))
          (:`OnCompleted`
            (`self.ClearAndEndAbility` :!label _label))
          (:`OnBlendOut`
            (goto _label))
          (:`OnInterrupted`
            (goto _label))
          (:`OnCancelled`
            (goto _label)))
        (else
          (`self.K2_EndAbility`))))))

(event `StartAttackTrace`
  (`NiagaraFunctionLibrary.SpawnSystemAttached` (`self.VFX`) (`Actor.RootComponent` (`self.GetAvatarActorFromActorInfo`)) "None" (0.0 0.0 0.0) (struct) "KeepRelativeOffset" true)
  (bind _returnvalue (`self.GenerateAttackTraceSockets` (`self.TipSocket`) true -50.0 10 300.0))
  (set `self.Last_TipSocketLocations` _returnvalue)
  (bind _returnvalue_2 (`self.GenerateAttackTraceSockets` (`self.TailSocket`) true -50.0 5))
  (set `self.Last_TailSocketLocations` _returnvalue_2)
  (bind _returnvalue_3 (`KismetSystemLibrary.K2_SetTimerDelegate` (delegate `TimerLineTrace`) 0.01 true))
  (set `self.Last_AttackTimerHandler` _returnvalue_3))

(event `TimerLineTrace`
  (bind _returnvalue (`self.GetAvatarActorFromActorInfo`))
  (`|ExecutionSequence`
    (:`then_0`
      (bind _returnvalue_2 (`self.GenerateAttackTraceSockets` (`self.TipSocket`) true -50.0 10 300.0))
      (bind _output_get (set `self.Current_TipSocketLocations` _returnvalue_2))
      (for (_array_element _array_index) _output_get
        (bind _outplayers (`AuraAbilitySystemLibrary.GetLivePlayerWithinRaycast` (`self.GetAvatarActorFromActorInfo`) (`self.IgnoreArray`) _array_element (`|GetArrayItem` (`self.Last_TipSocketLocations`) _array_index)))
        (for _array_element_2 _outplayers
          (bind _returnvalue_3 (`AuraAbilitySystemLibrary.IsFriendly` _array_element_2 (`self.GetAvatarActorFromActorInfo`)))
          (`KismetArrayLibrary.Array_Add` (`self.IgnoreArray`) _array_element_2)
          (if (not _returnvalue_3)
            (`self.K2_HasAuthority`
              (:`True`
                (`self.CauseDamage` _array_element_2)
                (bind _returnvalue_4 (message `EnemyInterface.GetCombatTarget` _returnvalue))
                (`self.K2_ExecuteGameplayCueWithParams` (struct :`TagName` "GameplayCue.MonkCombo") (`AbilitySystemBlueprintLibrary.MakeGameplayCueParameters` 0.0 0.0 (struct) (struct) (struct) (struct) (struct) (0.0 0.0 0.0) (0.0 0.0 0.0) null _returnvalue _returnvalue_4)))))))
      (`KismetArrayLibrary.Array_Clear` (`self.Last_TipSocketLocations`))
      (set `self.Last_TipSocketLocations` (`self.Current_TipSocketLocations`)))
    (:`then_1`
      (bind _returnvalue_5 (`self.GenerateAttackTraceSockets` (`self.TailSocket`) true -50.0 5))
      (bind _output_get_2 (set `self.Current_TrailSocketLocations` _returnvalue_5))
      (for (_array_element_3 _array_index_2) _output_get_2
        (bind _outplayers_2 (`AuraAbilitySystemLibrary.GetLivePlayerWithinRaycast` (`self.GetAvatarActorFromActorInfo`) (`self.IgnoreArray`) _array_element_3 (`|GetArrayItem` (`self.Last_TailSocketLocations`) _array_index_2)))
        (for _array_element_4 _outplayers_2
          (bind _returnvalue_6 (`AuraAbilitySystemLibrary.IsFriendly` _array_element_4 (`self.GetAvatarActorFromActorInfo`)))
          (`KismetArrayLibrary.Array_Add` (`self.IgnoreArray`) _array_element_4)
          (if (not _returnvalue_6)
            (`self.K2_HasAuthority`
              (:`True`
                (`self.CauseDamage` _array_element_4))))))
      (`KismetArrayLibrary.Array_Clear` (`self.Last_TailSocketLocations`))
      (set `self.Last_TailSocketLocations` (`self.Current_TrailSocketLocations`)))))

(fn `ClearAndEndAbility`
  (`KismetArrayLibrary.Array_Clear` (`self.Last_TipSocketLocations`))
  (`KismetArrayLibrary.Array_Clear` (`self.Last_TailSocketLocations`))
  (`KismetArrayLibrary.Array_Clear` (`self.Current_TipSocketLocations`))
  (`KismetSystemLibrary.K2_ClearAndInvalidateTimerHandle` (`self.Last_AttackTimerHandler`))
  (`self.K2_CommitAbilityCooldown` false)
  (`self.K2_EndAbility`))