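; Gameplay ability for Aura's Electrocute lightning skill, currently covering only cursor targeting and the hold-to-channel input lifecycle.
; On activation, a TargetDataUnderMouse task supplies the cursor hit result, which is stored along with the owning player controller.
; The mouse cursor is then hidden until a WaitInputRelease task fires, which shows it again and ends the ability.
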(event `self.K2_ActivateAbility`
  ;[0.05613 0 0.4072] 存储鼠标命中数据
  (bind (_asynctaskproxy _datahandle) (`TargetDataUnderMouse.CreateTargetDataUnderMouse`)
    (:`ValidData`
      (`self.StoreMouseInfo` (`AbilitySystemBlueprintLibrary.GetHitResultFromTargetData` _datahandle))
      (`self.StoreOwnerPlayerController`)
      (`|ExecutionSequence`
        (:`then_0`
          (set `PlayerController.bShowMouseCursor` false (`self.OwnerPlayerController`)))
        (:`then_1`
          (`AbilityTask_WaitInputRelease.WaitInputRelease` false
            (:`OnRelease`
              (set `PlayerController.bShowMouseCursor` true (`self.OwnerPlayerController`))
              (`self.K2_EndAbility`))))))))