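; Fireball actor for Aura's FireBlast ability that sweeps out around its ReturnTarget and comes back to explode.
; On authority, a timeline drives angle and radius from the initial forward, repositioning the ball around the target's current location each update.
; The smaller of the outgoing and ending radius curves shapes the out-and-back path.
; Past half the target angle and within ExplodeDistance of the target, it calls OnHit and destroys itself.
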(event `self.StartOutgoingTimeLine`
  (`/Engine/EditorBlueprintResources/ActorMacros.Switch Has Authority`
    (:`Authority`
      (set `self.InitialForward` (`self.GetActorForwardVector`))
      (set `self.TravelDistance` (`self.MaxFlyDistance`))
      ;[1 1 1] FireBall Fly Outgoing
      (bind (_direction _outgoingtrack_angle _outgoingtrack_radius _endgoingtrack_radius) (`Timeline|OutGoingTimeLine` :`NewTime` 4.0 :!label _label)
        (:`Update`
          (bind _returnvalue (`KismetMathLibrary.Lerp` 0.0 (`self.TargetAngle`) _outgoingtrack_angle))
          (set `self.CurrentAngle` _returnvalue)
          (bind _returnvalue_2 (`KismetMathLibrary.Lerp` 0.0 (`self.TravelDistance`) _outgoingtrack_radius))
          (set `self.CurrentRadius` _returnvalue_2)
          (`self.K2_SetActorLocation` (`AuraAbilitySystemLibrary.GetPositionByAngleAndRadius` (`self.K2_GetActorLocation` (`self.ReturnTarget`)) (`self.InitialForward`) _returnvalue (`KismetMathLibrary.FMin` _returnvalue_2 (`KismetMathLibrary.Lerp` (`self.TravelDistance`) 0.0 _endgoingtrack_radius))))
          (if (`self.IsClosedExploDistance`)
            (`self.OnHit`)
            (`self.K2_DestroyActor`)))))))

(event `EndFlying`
  (goto _label :!via `SetNewTime`))

(fn `IsClosedExploDistance`
  (returns (ReturnValue :type Boolean))
  (return (and (< (`KismetMathLibrary.VSize` (- (`self.K2_GetActorLocation`) (`self.K2_GetActorLocation` (`self.ReturnTarget`)))) (`self.ExplodeDistance`)) (> (`self.CurrentAngle`) (* (`self.TargetAngle`) 0.5)))))

(fn `UserConstructionScript`)