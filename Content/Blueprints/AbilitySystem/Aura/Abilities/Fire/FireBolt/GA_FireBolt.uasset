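; GA_FireBolt is the Fire Bolt gameplay ability that launches projectiles at the location under the cursor.
; On activation it commits cost and cooldown, caches the targeted location and actor, turns the avatar toward it and plays the cast montage.
; A montage gameplay event spawns the projectiles from the tagged combat socket, passing the hit actor as homing target and a distance-scaled, capped pitch.
; The ability ends when the montage finishes or is interrupted.
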(event `self.K2_ActivateAbility`
  ;[1 1 1] Commit节点同时提交了蓝耗和技能冷却这两个GE
  (`self.K2_CommitAbility`)
  (bind (_asynctaskproxy _datahandle) (`TargetDataUnderMouse.CreateTargetDataUnderMouse`)
    (:`ValidData`
      (bind (_bblockinghit _binitialoverlap _time _distance _location _impactpoint _normal _impactnormal _physmat _hitactor) (`GameplayStatics.BreakHitResult` (`AbilitySystemBlueprintLibrary.GetHitResultFromTargetData` _datahandle)))
      (set `self.ProjetileTargetLocation` _location)
      (set `self.MouseHitActor` _hitactor)
      (message `CombatInterface.UpdateFacingTarget` (`self.GetAvatarActorFromActorInfo`) (`self.ProjetileTargetLocation`))
      (`AbilityTask_PlayMontageAndWait.CreatePlayMontageAndWaitProxy` "None" "/Game/Blueprints/Character/Aura/Animation/AM_Cast_FireBolt.AM_Cast_FireBolt" 1.0 "None" false
        (:`then`
          (`AbilityTask_WaitGameplayEvent.WaitGameplayEvent` (struct :`TagName` "Event.Montage.FireBolt") null
            (:`EventReceived`
              (bind _returnvalue (message `CombatInterface.GetCombatSocketLocation` (`self.GetAvatarActorFromActorInfo`) (`self.Tag`)))
              (`self.SpawnProjectiles` (`self.ProjetileTargetLocation`) (`self.Tag`) (`self.MouseHitActor`) true (`KismetMathLibrary.FMin` (* (/ (`KismetMathLibrary.Vector_Distance` _returnvalue (`self.ProjetileTargetLocation`)) 1800.0) 45.0) 45.0)))))
        (:`OnCompleted`
          (`self.K2_EndAbility` :!label _label))
        (:`OnBlendOut`
          (goto _label))
        (:`OnInterrupted`
          (goto _label))
        (:`OnCancelled`
          (goto _label))))))