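; Arcane Shards gameplay ability: shows a magic circle on activation, then on input release bursts shards around the mouse-targeted location.
; A spawned BP_PointCollection supplies ground points at random yaw while the cast montage plays.
; The montage's gameplay event starts a looping timer that fires one shard per point as a GameplayCue, damaging nearby live targets with outward knockback.
; After the last point it destroys the collection and ends the ability.
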(event `self.K2_ActivateAbility`
  (`|ExecutionSequence`
    (:`then_0`
      (message `PlayerInterface.ShowMagicCircle` (`self.GetAvatarActorFromActorInfo`) null)
      (`TargetDataUnderMouse.CreateTargetDataUnderMouse`))
    (:`then_1`
      (`AbilityTask_WaitInputRelease.WaitInputRelease` false
        (:`OnRelease`
          (message `PlayerInterface.HideMagicCircle` (`self.GetAvatarActorFromActorInfo`))
          (bind (_asynctaskproxy _datahandle) (`TargetDataUnderMouse.CreateTargetDataUnderMouse`)
            (:`ValidData`
              (bind _output_get (set `self.MouseHitLocation` (`.ImpactPoint` (`GameplayStatics.BreakHitResult` (`AbilitySystemBlueprintLibrary.GetHitResultFromTargetData` _datahandle)))))
              (message `CombatInterface.UpdateFacingTarget` (`self.GetAvatarActorFromActorInfo`) _output_get)
              (bind _returnvalue (`|SpawnActorFromClass` "/Game/Blueprints/AbilitySystem/Aura/Arcane/ArcaneShards/BP_PointCollection.BP_PointCollection_C" (`KismetMathLibrary.MakeTransform` (`self.MouseHitLocation`)) "AlwaysSpawn" "MultiplyWithRoot" null null))
              (bind _output_get_2 (set `self.PointCollection` _returnvalue))
              (set `self.GroundPoints` (`PointCollection.GetGroundPoints` _output_get_2 (`self.MouseHitLocation`) (`self.NumPoints`) (`KismetMathLibrary.RandomFloatInRange` 0.0 360.0)))
              (`AbilityTask_PlayMontageAndWait.CreatePlayMontageAndWaitProxy` "None" "/Game/Blueprints/Character/Aura/Animation/AM_Cast_ArcaneShards_Montage.AM_Cast_ArcaneShards_Montage" 1.0 "None" false
                (:`then`
                  (`AbilityTask_WaitGameplayEvent.WaitGameplayEvent` (struct :`TagName` "Event.Montage.ArcaneShards") null
                    (:`EventReceived`
                      (bind _returnvalue_2 (`KismetSystemLibrary.K2_SetTimerDelegate` (delegate `SpawnShard`) (`self.ShardSpawnDeltatime`) true))
                      (set `self.SpawnPointTimer` _returnvalue_2)
                      (`self.SpawnShard`))))))))))))

(event `SpawnShard`
  (bind _returnvalue (`self.GetAvatarActorFromActorInfo`))
  (if (>= (`self.ShardCound`) (`self.NumPoints`))
    (`KismetSystemLibrary.K2_ClearAndInvalidateTimerHandle` (`self.SpawnPointTimer`))
    (`Actor.K2_DestroyActor` (`self.PointCollection`))
    (set `self.ShardCound` 0)
    (`KismetArrayLibrary.Array_Clear` (`self.GroundPoints`))
    (`KismetArrayLibrary.Array_Clear` (`self.ShardstTargets`))
    (`self.K2_EndAbility`)
    (else
      (set `self.PointLocation` (`SceneComponent.K2_GetComponentLocation` (`|GetArrayItem` (`self.GroundPoints`) (`self.ShardCound`))))
      (`/Engine/EditorBlueprintResources/StandardMacros.IncrementInt` (`self.ShardCound`)
        (:`  `
          (`self.K2_ExecuteGameplayCueWithParams` (struct :`TagName` "GameplayCue.ArcaneShards") (`AbilitySystemBlueprintLibrary.MakeGameplayCueParameters` 0.0 0.0 (struct) (struct) (struct) (struct) (struct) (`self.PointLocation`)))
          (bind _outplayers (`AuraAbilitySystemLibrary.GetLivePlayerWithinRadius` _returnvalue (`|MakeArray` _returnvalue) (`self.PointLocation`) 200.0))
          (bind _output_get (set `self.ShardstTargets` _outplayers))
          (for _array_element _output_get
            (bind _returnvalue_2 (- (`Actor.K2_GetActorLocation` _array_element) (`self.PointLocation`)))
            (`self.CauseDamage` _array_element (`self.PointLocation`) true _returnvalue_2 true _returnvalue_2 false 15.0)))))))