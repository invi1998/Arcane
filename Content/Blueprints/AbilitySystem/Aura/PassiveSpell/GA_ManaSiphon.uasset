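; GA_ManaSiphon is a passive spell gameplay ability that periodically applies the GE_ManaSiphon effect to its owner.
; On activation, if the avatar is not dead, it starts a looping one-second timer on the authority only.
; Each tick applies the effect at the current ability level, and ending the ability clears the timer.
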(event `self.K2_ActivateAbility`
  (bind _returnvalue (message `CombatInterface.IsDead` (`self.GetAvatarActorFromActorInfo`)))
  (if (not _returnvalue)
    (`self.K2_HasAuthority`
      (:`True`
        (bind _returnvalue_2 (`KismetSystemLibrary.K2_SetTimerDelegate` (delegate `AddMana`) 1.0 true))
        (set `self.AddManaTimer` _returnvalue_2)))))

(event `AddMana`
  (`self.BP_ApplyGameplayEffectToOwner` "/Game/Blueprints/AbilitySystem/Aura/PassiveSpell/GE_ManaSiphon.GE_ManaSiphon_C" (`self.GetAbilityLevel`)))

(event `self.K2_OnEndAbility`
  (params (bWasCancelled :type Boolean))
  (`KismetSystemLibrary.K2_ClearAndInvalidateTimerHandle` (`self.AddManaTimer`)))