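; GA_LifeSiphon is a passive Gameplay Ability that periodically restores health to its owner.
; On activation, it checks that the avatar is not dead, then starts a looping one-second timer.
; Each tick applies GE_LifeSiphon to the owner at the current ability level, and ending the ability clears the timer.
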(event `self.K2_ActivateAbility`
  (bind _returnvalue (message `CombatInterface.IsDead` (`self.GetAvatarActorFromActorInfo`)))
  (if (not _returnvalue)
    (bind _returnvalue_2 (`KismetSystemLibrary.K2_SetTimerDelegate` (delegate `AddHealth`) 1.0 true))
    (set `self.AddHealthTimer` _returnvalue_2)))

(event `AddHealth`
  (`self.BP_ApplyGameplayEffectToOwner` "/Game/Blueprints/AbilitySystem/Aura/PassiveSpell/GE_LifeSiphon.GE_LifeSiphon_C" (`self.GetAbilityLevel`)))

(event `self.K2_OnEndAbility`
  (params (bWasCancelled :type Boolean))
  (`KismetSystemLibrary.K2_ClearAndInvalidateTimerHandle` (`self.AddHealthTimer`)))