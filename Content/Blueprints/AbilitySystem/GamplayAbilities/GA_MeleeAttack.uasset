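; Melee attack gameplay ability that turns the avatar toward its combat target and plays a skeleton sword swing montage.
; A montage start event begins a fast looping trace timer; the end event clears it and ends the ability.
; Each tick samples points along the weapon socket's forward vector and line-traces to their previous positions to sweep the blade's path.
; Traces are debug-drawn, but their hits are not yet used.
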(event `self.K2_ActivateAbility`
  (bind _returnvalue (`self.GetAvatarActorFromActorInfo`))
  (bind _returnvalue_2 (message `EnemyInterface.GetCombatTarget` _returnvalue))
  (bind _ascombat_interface (cast `CombatInterface` _returnvalue))
  (bind _output_get (set `self.Combat` _ascombat_interface))
  (`CombatInterface.UpdateFacingTarget` _output_get (`Actor.K2_GetActorLocation` _returnvalue_2))
  (`AbilityTask_PlayMontageAndWait.CreatePlayMontageAndWaitProxy` "None" "/Game/Blueprints/Character/Skeleton_Sword/Animation/AM_SkeletonSwordRightAttack.AM_SkeletonSwordRightAttack"
    (:`then`
      (`AbilityTask_WaitGameplayEvent.WaitGameplayEvent` (struct :`TagName` "Event.Montage.Attack.SworlAttackStart") null
        (:`then`
          (`AbilityTask_WaitGameplayEvent.WaitGameplayEvent` (struct :`TagName` "Event.Montage.Attack.SworlAttackEnd") null
            (:`EventReceived`
              (`KismetSystemLibrary.K2_ClearAndInvalidateTimerHandle` (`self.AttackTimerHandle`))
              (`self.K2_EndAbility`))))
        (:`EventReceived`
          (`self.AttackStart`))))))

(event `AttackStart`
  (set `self.LastAttackTracePoint` (`self.Get Sword Attack Trace Point`))
  (bind _returnvalue (`KismetSystemLibrary.K2_SetTimerDelegate` (delegate `AttackDrawTrace`) 0.01 true))
  (set `self.AttackTimerHandle` _returnvalue))

(event `AttackDrawTrace`
  (bind _output_get (set `self.CurrentAttackTracePoint` (`self.Get Sword Attack Trace Point`)))
  (for (_array_element _array_index) _output_get
    (`KismetSystemLibrary.LineTraceMulti` :`Start` _array_element :`End` (`|GetArrayItem` (`self.LastAttackTracePoint`) _array_index) :`TraceChannel` "TraceTypeQuery1" :`DrawDebugType` "ForDuration" :`TraceColor` (struct :`R` 1.0 :`B` 0.490177 :`A` 1.0) :`DrawTime` 1.0))
  (`KismetArrayLibrary.Array_Clear` (`self.LastAttackTracePoint`))
  (set `self.LastAttackTracePoint` (`self.CurrentAttackTracePoint`)))

(fn `Get Sword Attack Trace Point`
  (returns (TraceStartEnd :type "Array of Vector Structure"))
  (locals (AttackTracePoint :type "Array of Vector Structure") (StartVec :type "Vector Structure" :default (0.0 0.0 0.0)) (EndVec :type "Vector Structure") (DirVec :type "Vector Structure" :default (0.0 0.0 0.0)) (OutVec :type "Array of Vector Structure"))
  (bind _returnvalue (`self.GetAvatarActorFromActorInfo`))
  (bind _returnvalue_2 (message `CombatInterface.GetCombatSocketLocation` _returnvalue))
  (set `local.StartVec` _returnvalue_2)
  (bind _returnvalue_3 (message `CombatInterface.GetCombatSocketForward` _returnvalue))
  (set `local.DirVec` _returnvalue_3)
  (for _index (range 9)
    (`KismetArrayLibrary.Array_Add` (`local.OutVec`) (+ (`local.StartVec`) (* (* _index 15.0) (`local.DirVec`)))))
  (return (`local.OutVec`)))