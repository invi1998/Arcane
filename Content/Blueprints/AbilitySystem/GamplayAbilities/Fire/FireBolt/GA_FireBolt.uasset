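; Fire Bolt gameplay ability, meant to cast a projectile toward the point under the mouse.
; On activation it uses a TargetDataUnderMouse task to store the hit location, then casts the avatar to CombatInterface, where the live chain stops.
; A disconnected chain would play the cast montage, wait for its Fire Bolt gameplay event, spawn the projectile at that location and end the ability, but it never runs.
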(event `self.K2_ActivateAbility`
  (bind (_asynctaskproxy _datahandle) (`TargetDataUnderMouse.CreateTargetDataUnderMouse`)
    (:`ValidData`
      (set `self.ProjetileTargetLocation` (`.Location` (`GameplayStatics.BreakHitResult` (`AbilitySystemBlueprintLibrary.GetHitResultFromTargetData` _datahandle))))
      (cast `CombatInterface` (`self.GetAvatarActorFromActorInfo`)))))