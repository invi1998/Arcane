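; Melee sword attack gameplay ability that turns the avatar toward its combat target and plays a random attack montage.
; A montage start event begins a looping timer that samples points along the weapon socket's forward direction and raycasts between previous and current positions to catch the swing.
; Each living player hit takes damage and joins an ignore list, preventing repeat hits.
; The end event stops tracing and ends the ability, as does montage completion or interruption.
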(event `self.K2_ActivateAbility`
  (bind _returnvalue (`self.GetAvatarActorFromActorInfo`))
  (set `self.IgmoreArray` (`|MakeArray` _returnvalue))
  (bind _returnvalue_2 (message `EnemyInterface.GetCombatTarget` _returnvalue))
  (bind _ascombat_interface (cast `CombatInterface` _returnvalue))
  (bind _output_get (set `self.Combat` _ascombat_interface))
  (`CombatInterface.UpdateFacingTarget` _output_get (`Actor.K2_GetActorLocation` _returnvalue_2))
  (bind _returnvalue_3 (message `CombatInterface.GetRandomAttackMontage` (`self.GetAvatarActorFromActorInfo`)))
  (bind (_montage _montagetag) (break `TaggedMontage` _returnvalue_3))
  (`AbilityTask_PlayMontageAndWait.CreatePlayMontageAndWaitProxy` "None" _montage 1.0 "None" false
    (:`then`
      (`AbilityTask_WaitGameplayEvent.WaitGameplayEvent` (struct :`TagName` "Event.Montage.Attack.SworlAttackStart") null
        (:`then`
          (`AbilityTask_WaitGameplayEvent.WaitGameplayEvent` (struct :`TagName` "Event.Montage.Attack.SworlAttackEnd") null
            (:`EventReceived`
              (`KismetSystemLibrary.K2_ClearAndInvalidateTimerHandle` (`self.AttackTimerHandle`))
              (`KismetArrayLibrary.Array_Clear` (`self.IgmoreArray`))
              (`self.K2_EndAbility` :!label _label))))
        (:`EventReceived`
          (`self.AttackStart` _montagetag))))
    (:`OnCompleted`
      (goto _label))
    (:`OnInterrupted`
      (goto _label))
    (:`OnCancelled`
      (goto _label))))

(event `AttackStart`
  (params (Tag :type "GameplayTag Structure"))
  (set `self.LastAttackTracePoint` (`self.Get Sword Attack Trace Point` Tag))
  (bind _returnvalue (`KismetSystemLibrary.K2_SetTimerDelegate` (delegate `AttackDrawTrace`) 0.01 true))
  (set `self.AttackTimerHandle` _returnvalue))

(event `AttackDrawTrace`
  (bind _output_get (set `self.CurrentAttackTracePoint` (`self.Get Sword Attack Trace Point` (stale `AttackStart` Tag))))
  (for (_array_element _array_index) _output_get
    (bind _outplayers (`AuraAbilitySystemLibrary.GetLivePlayerWithinRaycast` (`self.GetAvatarActorFromActorInfo`) (`self.IgmoreArray`) _array_element (`|GetArrayItem` (`self.LastAttackTracePoint`) _array_index)))
    (for _array_element_2 _outplayers
      (`KismetArrayLibrary.Array_Add` (`self.IgmoreArray`) _array_element_2)
      (`self.CauseDamage` _array_element_2)))
  (`KismetArrayLibrary.Array_Clear` (`self.LastAttackTracePoint`))
  (set `self.LastAttackTracePoint` (`self.CurrentAttackTracePoint`)))

(fn `Get Sword Attack Trace Point`
  (params (inMontageTag :type "GameplayTag Structure"))
  (returns (TraceStartEnd :type "Array of Vector Structure"))
  (locals (AttackTracePoint :type "Array of Vector Structure") (StartVec :type "Vector Structure" :default (0.0 0.0 0.0)) (EndVec :type "Vector Structure") (DirVec :type "Vector Structure" :default (0.0 0.0 0.0)) (OutVec :type "Array of Vector Structure") (RightWeapon :type "GameplayTag Structure" :default (struct :`TagName` "Montage.Attack.RightWeaponLeftSwing")))
  (bind _returnvalue (`self.GetAvatarActorFromActorInfo`))
  (bind _returnvalue_2 (message `CombatInterface.GetCombatSocketLocation` _returnvalue inMontageTag))
  (set `local.StartVec` _returnvalue_2)
  (bind _returnvalue_3 (message `CombatInterface.GetCombatSocketForward` _returnvalue inMontageTag))
  (set `local.DirVec` _returnvalue_3)
  (for _index (range 9)
    (`KismetArrayLibrary.Array_Add` (`local.OutVec`) (+ (`local.StartVec`) (* (* _index 15.0) (`local.DirVec`)))))
  (return (`local.OutVec`)))