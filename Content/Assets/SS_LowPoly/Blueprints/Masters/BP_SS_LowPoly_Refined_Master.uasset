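; Master actor for refined low-poly props that animates its mesh into view on BeginPlay.
; The mesh is hidden for a short random delay, then shown as a timeline drives actor scale and adds a local movement offset on each update.
; Query and physics collision is enabled on the mesh once the timeline finishes.
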(event `self.ReceiveBeginPlay`
  (bind _sm_lp_refined (`self.SM_LP_Refined`))
  (`SceneComponent.SetVisibility` _sm_lp_refined false false)
  (`KismetSystemLibrary.Delay` (* (`KismetMathLibrary.RandomFloat`) 0.5))
  (`SceneComponent.SetVisibility` _sm_lp_refined true false)
  (bind (_direction _move_out _scale) (`Timeline|Timeline` :!via `PlayFromStart`)
    (:`Update`
      (`self.SetActorScale3D` (`KismetMathLibrary.Conv_DoubleToVector` _scale))
      (`self.K2_AddActorLocalOffset` _move_out))
    (:`Finished`
      (`PrimitiveComponent.SetCollisionEnabled` _sm_lp_refined "QueryAndPhysics"))))

(fn `UserConstructionScript`)