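; Master Blueprint for a low-poly resource node that breaks apart on a single click and spawns refined resource actors.
; The click hides the static mesh, crumbles the hidden Geometry Collection with physics, adds a Niagara effect and stops the glow.
; It spawns SpawnAmount copies of the child actor's class with random yaw.
; After a delay, a timeline sinks and scales the node before it is destroyed.
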(event `self.ReceiveBeginPlay`
  (`SceneComponent.SetVisibility` (`self.GC_LP_Pieces`) false false))

(event `self.ReceiveActorOnClicked`
  (params (ButtonPressed :type "Key Structure"))
  (bind _sm_lp_node (`self.SM_LP_Node`))
  (bind _gc_lp_pieces (`self.GC_LP_Pieces`))
  ;[1 1 1] Input
  (`/Engine/EditorBlueprintResources/StandardMacros.Do N` 1
    (:`Exit`
      ;[1 1 1] Break Node
      (`SceneComponent.SetVisibility` _sm_lp_node false false)
      (`PrimitiveComponent.SetCollisionEnabled` _sm_lp_node "NoCollision")
      (`SceneComponent.SetVisibility` _gc_lp_pieces true false)
      (`PrimitiveComponent.SetSimulatePhysics` _gc_lp_pieces true)
      (`GeometryCollectionComponent.CrumbleCluster` _gc_lp_pieces 0)
      (`AddComponent|NODE_AddNiagaraComponent-1`)
      (`ActorComponent.Deactivate` (`self.NS_Glow`))
      ;[1 1 1] Spawn Resource
      (for _ (range (`self.SpawnAmount`))
        (bind _returnvalue (`|SpawnActorFromClass` (`ChildActorComponent.ChildActorClass` (`self.BP_LP_Refined`)) (`SceneComponent.GetRelativeTransform` (`self.DefaultSceneRoot`)) "Undefined" "SelectDefaultAtRuntime" null null))
        (`self.K2_SetActorRotation` _returnvalue (`KismetMathLibrary.MakeRotator` 0.0 0.0 (`KismetMathLibrary.RandomFloatInRange` 0.0 360.0)) false))
      ;[1 1 1] Clean up
      (`KismetSystemLibrary.Delay` 8.0)
      (bind (_direction _scale_down _movedown) (`Timeline|Timeline` :!via `PlayFromStart`)
        (:`Update`
          (`self.K2_AddActorWorldOffset` _movedown false true)
          (`self.SetActorScale3D` (`KismetMathLibrary.Conv_DoubleToVector` _scale_down))
          (`KismetSystemLibrary.Delay` 1.0)
          (`self.K2_DestroyActor`))))))

(fn `Break Node`
  (params (SM_Mineral :type "StaticMeshComponent Object Reference") (GC_MineralPieces :type "GeometryCollectionComponent Object Reference") (NS_Glow :type "NiagaraComponent Object Reference"))
  ;[1 1 1] Break Node
  (`SceneComponent.SetVisibility` SM_Mineral false false)
  (`PrimitiveComponent.SetCollisionEnabled` SM_Mineral "NoCollision")
  (`SceneComponent.SetVisibility` GC_MineralPieces true false)
  (`PrimitiveComponent.SetSimulatePhysics` GC_MineralPieces true)
  (`GeometryCollectionComponent.CrumbleCluster` GC_MineralPieces 0)
  (`AddComponent|NODE_AddNiagaraComponent-0`)
  (`ActorComponent.Deactivate` NS_Glow))

(fn `UserConstructionScript`)