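; BP_Homming_Projectile10 is a homing projectile with a Niagara trail that chases actors tagged Projectile_Target.
; BeginPlay randomizes homing acceleration from HomingSpeed, then loops on a short delay to re-lock ProjectileMovement onto FindTarget's result.
; FindTarget scans tagged actors by distance, but MinDistance is never reset, so the target changes only when one beats the closest distance recorded.
; Hitting a tagged actor spawns Hitfx along the impact normal and destroys the projectile.
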(event `self.ReceiveBeginPlay`
  (bind _projectile_trail2 (`self.Projectile_Trail2`))
  (bind _homing_speed (`self.Homing_Speed`))
  (`NiagaraFunctionLibrary.SpawnSystemAttached` (`NiagaraComponent.GetAsset` _projectile_trail2) _projectile_trail2 "None" (0.0 0.0 0.0) (struct) "KeepRelativeOffset" false true "AutoRelease")
  (set `ProjectileMovementComponent.HomingAccelerationMagnitude` (`KismetMathLibrary.RandomFloatInRange` (/ _homing_speed 2.0) _homing_speed) (`self.ProjectileMovement`))
  (`self.Lock` :!label _label)
  (`KismetSystemLibrary.Delay` 0.2)
  (goto _label))

(event `Lock`
  (bind _projectilemovement (`self.ProjectileMovement`))
  (bind _targetwww (`self.Find_Target`))
  (set `ProjectileMovementComponent.HomingTargetComponent` _targetwww _projectilemovement)
  (set `ProjectileMovementComponent.bIsHomingProjectile` true _projectilemovement))

(event `self.Sphere.OnComponentHit`
  (params (HitComponent :type "PrimitiveComponent Object Reference") (OtherActor :type "Actor Object Reference") (OtherComp :type "PrimitiveComponent Object Reference") (NormalImpulse :type "Vector Structure") (Hit :type "HitResult Structure (by ref)"))
  (bind (_bblockinghit _binitialoverlap _time _distance _location _impactpoint _normal _impactnormal) (`GameplayStatics.BreakHitResult` Hit))
  (if (`self.ActorHasTag` OtherActor "Projectile_Target")
    (`NiagaraFunctionLibrary.SpawnSystemAtLocation` (`self.Hitfx`) _location (`KismetMathLibrary.Conv_VectorToRotator` _impactnormal))
    (`self.K2_DestroyActor`)))

(fn `Find_Target`
  (returns (Targetwww :type "SceneComponent Object Reference"))
  (bind _outactors (`GameplayStatics.GetAllActorsOfClassWithTag` "/Script/Engine.Actor" "Projectile_Target"))
  (for _array_element _outactors
    (bind _returnvalue (`KismetMathLibrary.VSize` (- (`self.K2_GetActorLocation` _array_element) (`self.K2_GetActorLocation`))))
    (if (< _returnvalue (`self.MinDistance`))
      (set `self.MinDistance` _returnvalue)
      (set `self.Target` _array_element)))
  (return (`self.GetComponentByClass` (`self.Target`) "/Script/Engine.SceneComponent")))

(fn `UserConstructionScript`)